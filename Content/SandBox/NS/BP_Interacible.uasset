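; BP_Interacible is an interactable actor that registers itself with BP_ThirdPersonCharacter while that character overlaps its box trigger.
; The construction script configures the mesh, trigger and UI component from variables, sizing the box uniformly from TriggerRadius.
; Overlap begin and end call AddInteraction and RemoveInteraction on the character, and ToggleUI exposes prompt visibility.
; Interact is a placeholder that stores the interacting character and prints a debug string.
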(event OnComponentBeginOverlap(InteractTrigger)
  (params (OverlappedComponent :type Primitive%20Component%20Object%20Reference) (OtherActor :type Actor%20Object%20Reference) (OtherComp :type Primitive%20Component%20Object%20Reference) (OtherBodyIndex :type Integer) (bFromSweep :type Boolean) (SweepResult :type Hit%20Result%20Structure%20%28by%20ref%29))
  (bind _asbp_third_person_character (Utilities|Casting|CastToBP_ThirdPersonCharacter OtherActor))
  (Default|AddInteraction _asbp_third_person_character self))

(event OnComponentEndOverlap(InteractTrigger)
  (params (OverlappedComponent :type Primitive%20Component%20Object%20Reference) (OtherActor :type Actor%20Object%20Reference) (OtherComp :type Primitive%20Component%20Object%20Reference) (OtherBodyIndex :type Integer))
  (bind _asbp_third_person_character (Utilities|Casting|CastToBP_ThirdPersonCharacter OtherActor))
  (Default|RemoveInteraction _asbp_third_person_character self))

(fn ConstructionScript
  (CallFunction|SetupMesh)
  (CallFunction|SetupTrigger)
  (CallFunction|SetupUI))

(fn SetupMesh
  (Components|StaticMesh|SetStaticMesh (Variables|Default|GetInteractMesh) (Variables|Setup|GetInteractionMesh))
  (Transformation|SetRelativeTransform (Variables|Default|GetInteractMesh) (Variables|Setup|GetMeshTransform) false false))

(fn SetupTrigger
  (Components|Box|SetBoxExtent (Variables|Default|GetInteractTrigger) (Math|Conversions|ToVector(Float) (Variables|Setup|GetTriggerRadius)) true)
  (Transformation|SetRelativeLocation (Variables|Default|GetInteractTrigger) (Variables|Setup|GetTriggerLocation) false false))

(fn SetupUI
  (Transformation|SetRelativeLocation (Variables|Default|GetInteractUI) (Variables|Setup|GetUILocation) false false))

(fn ToggleUI
  (params (bVisible :type Boolean))
  (Rendering|SetVisibility (Variables|Default|GetInteractUI) bVisible false))

(fn Interact
  (params (Character :type BP%20Third%20Person%20Character%20Object%20Reference))
  (Variables|Default|SetInteractCharacter Character)
  (Development|PrintString "Interaction Result"))