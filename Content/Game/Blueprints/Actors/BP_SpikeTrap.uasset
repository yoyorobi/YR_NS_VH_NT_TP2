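; BP_SpikeTrap is a trap actor that damages the third-person player character when it overlaps the trap's Box.
; Tick binds the Box's begin-overlap event whenever Danger is true, with no unbind when it turns false.
; The overlap handler reaches the health component through the character's BP_PlayerState, applies DamageAmount and plays 2D stabbing and scream sounds.
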(event Custom|OnComponentBeginOverlap_Événement
  (params (OverlappedComponent :type Primitive%20Component%20Object%20Reference) (OtherActor :type Actor%20Object%20Reference) (OtherComp :type Primitive%20Component%20Object%20Reference) (OtherBodyIndex :type Integer) (bFromSweep :type Boolean) (SweepResult :type Hit%20Result%20Structure%20%28by%20ref%29))
  (bind _asbp_third_person_character (Utilities|Casting|CastToBP_ThirdPersonCharacter OtherActor))
  (bind _asbp_player_state (Utilities|Casting|CastToBP_PlayerState (Variables|/Script/Engine.Pawn|GetPlayerState _asbp_third_person_character)))
  (Default|TakeDamage (Variables|/Game/Game/Blueprints/PlayerStates/BP_PlayerState.BP_PlayerState_C|GetAC_Health _asbp_player_state) (Variables|Default|GetDamage%20Amount))
  (Audio|PlaySound2D "/Game/Game/SFX/Stabbing.Stabbing" 1.0 1.0 0.0 0 0)
  (Audio|PlaySound2D "/Game/Game/SFX/ManScream.ManScream" 1.0 1.0 0.0 0 0))

(event EventTick
  (params (DeltaSeconds :type Float%20%28single-precision%29))
  (if (Variables|Default|GetDanger)
    (Collision|AssignOnComponentBeginOverlap (Variables|Default|GetBox) (delegate Custom|OnComponentBeginOverlap_Événement))))

(fn ConstructionScript)